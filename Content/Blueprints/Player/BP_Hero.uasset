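; BP_Hero is the player hero Blueprint that owns the player HUD and handles weapon switching input.
; On BeginPlay it creates the UMG_PlayerUI widget, stores it as UI and adds it to the viewport.
; NextWeapon and PreviousWeapon input actions call the matching switch functions, print a debug string, then both tell the UI to refresh its circle display through UpdateCircle.
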(event `self.ReceiveBeginPlay`
  (bind _returnvalue (`|CreateWidget` "/Game/Blueprints/UI/UMG_PlayerUI.UMG_PlayerUI_C"))
  (set `self.UI` _returnvalue)
  (`UserWidget.AddToViewport` _returnvalue 0))

(event `InputAction|NextWeapon`
  (params (Key :type "Key Structure"))
  (:`Pressed`
    (`self.NextWeapon`)
    (`KismetSystemLibrary.PrintString` "adelante")
    (`/Game/Blueprints/UI/UMG_PlayerUI.UpdateCircle` (`self.UI`) :!label _label)))

(event `InputAction|PreviousWeapon`
  (params (Key :type "Key Structure"))
  (:`Pressed`
    (`self.PreviousWeapon`)
    (`KismetSystemLibrary.PrintString` "atras")
    (goto _label)))

(fn `UserConstructionScript`)